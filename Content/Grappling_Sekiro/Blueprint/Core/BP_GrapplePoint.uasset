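; BP_GrapplePoint is a grapple target that shows a detection widget to the player.
; Activate and Deactivate toggle the widget, and while active, Tick scales its fill by player distance, turning it green within throw range.
; Use plays the widget's use animation and locks the point for two seconds before reactivating.
; An inner DeactivateZone disables the Detection collision while the player overlaps it.
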(event `self.ReceiveBeginPlay`
  (bind _aswbp_detection_node (cast `/Game/Grappling_Sekiro/Blueprint/UI/WBP_DetectionNode` (`WidgetComponent.GetUserWidgetObject` (`self.Widget`))))
  (bind _output_get (set `self.WidgetRef` _aswbp_detection_node))
  (`Widget.SetVisibility` _output_get "Hidden"))

(event `self.ReceiveTick`
  (params (DeltaSeconds :type "Float (single-precision)"))
  (if (and (`self.bActive`) (not (`self.bUsed`)))
    (`self.CheckDistanceFromPlayer`)))

(event `self.DeactivateZone.OnComponentBeginOverlap`
  (params (OverlappedComponent :type "PrimitiveComponent Object Reference") (OtherActor :type "Actor Object Reference") (OtherComp :type "PrimitiveComponent Object Reference") (OtherBodyIndex :type Integer) (bFromSweep :type Boolean) (SweepResult :type "HitResult Structure (by ref)"))
  (if (== OtherActor (`self.PlayerRef`))
    (`PrimitiveComponent.SetCollisionEnabled` (`self.Detection`) "NoCollision")))

(event `self.DeactivateZone.OnComponentEndOverlap`
  (params (OverlappedComponent :type "PrimitiveComponent Object Reference") (OtherActor :type "Actor Object Reference") (OtherComp :type "PrimitiveComponent Object Reference") (OtherBodyIndex :type Integer))
  (if (== OtherActor (`self.PlayerRef`))
    (`PrimitiveComponent.SetCollisionEnabled` (`self.Detection`) "QueryOnly")))

(fn `Activate`
  (params (Player :type "/Game/Grappling_Sekiro/Blueprint/Core/BP_PawnSekiro Object Reference"))
  (if (not (`self.bUsed`))
    (set `self.PlayerRef` Player)
    (set `self.bActive` true)
    (`Widget.SetVisibility` (`self.WidgetRef`) "Visible")))

(fn `CheckDistanceFromPlayer`
  (bind _playerref (`self.PlayerRef`))
  (bind _returnvalue (`KismetMathLibrary.MapRangeClamped` (`KismetMathLibrary.VSize` (- (`self.K2_GetActorLocation` (`self.PlayerRef`)) (`self.K2_GetActorLocation`))) (`/Game/Grappling_Sekiro/Blueprint/Core/BP_PawnSekiro.GrappleThrowDistance` _playerref) (`/Game/Grappling_Sekiro/Blueprint/Core/BP_PawnSekiro.DetectionRadius` _playerref) 80.0 10.0))
  (`Image.SetBrushSize` (`/Game/Grappling_Sekiro/Blueprint/UI/WBP_DetectionNode.Filling` (`self.WidgetRef`)) (`KismetMathLibrary.MakeVector2D` _returnvalue _returnvalue))
  (`Image.SetColorAndOpacity` (`/Game/Grappling_Sekiro/Blueprint/UI/WBP_DetectionNode.Filling` (`self.WidgetRef`)) (select `bool` (== _returnvalue 80.0) :`false` (struct :`R` 0.244792 :`G` 0.244792 :`B` 0.244792 :`A` 1.0) :`true` (struct :`R` 0.1841 :`G` 0.630208 :`B` 0.206321 :`A` 1.0) :!type "LinearColor Structure")))

(fn `Deactivate`
  (bind _widgetref (`self.WidgetRef`))
  (if (not (`self.bUsed`))
    (set `self.bActive` false)
    (`Widget.SetVisibility` _widgetref "Hidden")
    (`UserWidget.StopAllAnimations` _widgetref)))

(fn `Reactivate`
  (set `self.bUsed` false))

(fn `Use`
  (bind _widgetref (`self.WidgetRef`))
  (set `self.bUsed` true)
  (`UserWidget.PlayAnimation` _widgetref (`/Game/Grappling_Sekiro/Blueprint/UI/WBP_DetectionNode.NodeUse` _widgetref) 0.0 1 "Forward" 1.0 true)
  (`KismetSystemLibrary.K2_SetTimer` null "Reactivate" 2.0))

(fn `UserConstructionScript`)